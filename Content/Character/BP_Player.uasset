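; Player character with Enhanced Input movement, look and jump, plus a sword attack, two abilities and health.
; Attack animates the sword through a timeline and applies delayed box-trace damage; E damages pawns along a long, narrow box trace.
; Q line-traces to spawn BP_ZonaCuracion at the hit point, and key 1 plays a sword flourish.
; Incoming damage is clamped and throttled by DoOnce, Curar restores capped HP, and defeat only prints a message.
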(event Custom|MoverEspada
  (Utilities|FlowControl|DoOnce false :!label _label
    (:Completed
      (bind _newtrack_0 (Timeline|espda PlayFromStart)
        (:Update
          (Transformation|SetRelativeRotation (Variables|Default|GetespadaOrigin) (Math|Rotator|Lerp(Rotator) "0, 0, 0" "-70.000000,0.000000,0.000000" _newtrack_0) false false))
        (:Finished
          (goto _label Reset))))))

(event Input|EnhancedActionEvents|EnhancedInputActionIA_Moverse
  (params (ActionValue :type Vector%202D%20Structure) (ElapsedSeconds :type Float%20%28double-precision%29) (TriggeredSeconds :type Float%20%28double-precision%29) (InputAction :type Input%20Action%20Object%20Reference :default "/Game/Character/Input/Actions/IA_Moverse.IA_Moverse"))
  ;[0.15 0.15 0.15 0.5] sistema de movimiento
  (CallFunction|Moverse (.x ActionValue) (.y ActionValue)))

(event Input|EnhancedActionEvents|EnhancedInputActionIA_Mirar
  (params (ActionValue :type Vector%202D%20Structure) (ElapsedSeconds :type Float%20%28double-precision%29) (TriggeredSeconds :type Float%20%28double-precision%29) (InputAction :type Input%20Action%20Object%20Reference :default "/Game/Character/Input/Actions/IA_Mirar.IA_Mirar"))
  ;[0.15 0.15 0.15 0.5] sistema de movimiento
  (CallFunction|Mirar (.x ActionValue) (.y ActionValue)))

(event Input|EnhancedActionEvents|EnhancedInputActionIA_Ataque
  (params (ActionValue :type Boolean) (ElapsedSeconds :type Float%20%28double-precision%29) (TriggeredSeconds :type Float%20%28double-precision%29) (InputAction :type Input%20Action%20Object%20Reference :default "/Game/Character/Input/Actions/IA_Ataque.IA_Ataque"))
  (bind _mesh (Variables|Character|GetMesh))
  (bind _returnvalue (Transformation|GetWorldLocation _mesh))
  (:Triggered
    (CallFunction|MoverEspada))
  (:Started
    (Utilities|FlowControl|Delay 0.2)
    (bind (_outhits _returnvalue_2) (Class|KismetSystemLibrary|BoxTraceMultiforObjects _returnvalue (+ _returnvalue (* (Math|Vector|GetForwardVector _mesh) 3e+02)) "50.000000,50.000000,50.000000" "0, 0, 0" (Utilities|Array|MakeArray "ObjectTypeQuery3") false (Utilities|Array|MakeArray self) "ForDuration" true))
    (bind _array_element (Utilities|Array|ForEachLoopwithBreak _outhits)
      (:LoopBody
        (if _returnvalue_2
          (Game|Damage|ApplyDamage (.HitActor (Collision|BreakHitResult _array_element)) 1.0 0 0))))))

(event Input|EnhancedActionEvents|EnhancedInputActionIA_Saltar
  (params (ActionValue :type Boolean) (ElapsedSeconds :type Float%20%28double-precision%29) (TriggeredSeconds :type Float%20%28double-precision%29) (InputAction :type Input%20Action%20Object%20Reference :default "/Game/Character/Input/Actions/IA_Saltar.IA_Saltar"))
  (:Started
    (Character|Jump)))

(event Input|EnhancedActionEvents|EnhancedInputActionIA_Q
  (params (ActionValue :type Boolean) (ElapsedSeconds :type Float%20%28double-precision%29) (TriggeredSeconds :type Float%20%28double-precision%29) (InputAction :type Input%20Action%20Object%20Reference :default "/Game/Character/Input/Actions/IA_Q.IA_Q"))
  (bind _origenq (Variables|Default|GetorigenQ))
  (bind _returnvalue (Transformation|GetWorldLocation _origenq))
  (:Started
    (bind (_outhit _returnvalue_2) (Collision|LineTraceByChannel _returnvalue (+ _returnvalue (* (Math|Vector|GetForwardVector _origenq) 1e+03)) "TraceTypeQuery1" false 0 "ForDuration"))
    (if _returnvalue_2
      (Game|SpawnActorfromClass "/Game/Features/BP_ZonaCuracion.BP_ZonaCuracion_C" (Math|Transform|MakeTransform (.Location (Collision|BreakHitResult _outhit)) "0, 0, 0" "1.000000,1.000000,1.000000") "Undefined" "MultiplyWithRoot" 0 0))))

(event Input|EnhancedActionEvents|EnhancedInputActionIA_E
  (params (ActionValue :type Boolean) (ElapsedSeconds :type Float%20%28double-precision%29) (TriggeredSeconds :type Float%20%28double-precision%29) (InputAction :type Input%20Action%20Object%20Reference :default "/Game/Character/Input/Actions/IA_E.IA_E"))
  (bind _origene (Variables|Default|GetOrigenE))
  (bind _returnvalue (Transformation|GetWorldLocation _origene))
  (:Started
    (bind (_outhits _returnvalue_2) (Class|KismetSystemLibrary|BoxTraceMultiforObjects _returnvalue (+ _returnvalue (* (Math|Vector|GetForwardVector _origene) 1.3e+03)) "10.000000,10.000000,10.000000" "0, 0, 0" (Utilities|Array|MakeArray "ObjectTypeQuery3") false (Utilities|Array|MakeArray self) "ForDuration" true))
    (bind _array_element (Utilities|Array|ForEachLoopwithBreak _outhits)
      (:LoopBody
        (if _returnvalue_2
          (Game|Damage|ApplyDamage (.HitActor (Collision|BreakHitResult _array_element)) 1.0 0 0))))))

(event Game|Damage|EventAnyDamage
  (params (Damage :type Float%20%28single-precision%29) (DamageType :type Damage%20Type%20Object%20Reference) (InstigatedBy :type Controller%20Object%20Reference) (DamageCauser :type Actor%20Object%20Reference))
  (Utilities|FlowControl|DoOnce false :!label _label
    (:Completed
      (bind _output_get (Variables|Default|SetHP_Player (- (Variables|Default|GetHP_Player) (Math|Float|Clamp(Float) Damage))))
      (if (== _output_get 0.0)
        (Development|PrintString "perdiste")
        (else
          (Development|PrintString (Utilities|String|ToString(Float) _output_get))
          (Utilities|FlowControl|Delay 0.2)
          (goto _label Reset))))))

(event EventBeginPlay
  ;[0.15 0.15 0.15 0.5] begin play
  (Input|AddMappingContext (PlayerController|LocalPlayerSubsystems|GetEnhancedInputLocalPlayerSubsystem (Game|GetPlayerController 0)) "/Game/Character/Input/IMC_Controles.IMC_Controles" 0 "(bIgnoreAllPressedKeysUntilRelease=True,bForceImmediately=False,bNotifyUserSettings=False)")
  (bind _returnvalue (Actor|GetActorOfClass "/Game/Character/Peronsaje_Q/BP_AuraLuzSanacion.BP_AuraLuzSanacion_C"))
  (Variables|Default|SetAuraLuzQ _returnvalue))

(event Input|KeyboardEvents|1
  (params (Key :type Key%20Structure :default "None"))
  ;[0.15 0.15 0.15 0.5] guiño tin tin tinnn
  (:Pressed
    (Utilities|FlowControl|DoOnce false :!label _label
      (:Completed
        (bind _newtrack_0 (Timeline|Timeline PlayFromStart)
          (:Update
            (Transformation|SetRelativeRotation (Variables|Default|GetespadaOrigin) (Math|Rotator|Lerp(Rotator) "0, 0, 0" "0.000000,0.000000,-60.000000" _newtrack_0) false false))
          (:Finished
            (goto _label Reset)))))))

(fn ConstructionScript)

(fn Mirar
  (params (Yaw :type Float%20%28double-precision%29) (Pitch :type Float%20%28double-precision%29))
  (Pawn|Input|AddControllerYawInput Yaw)
  (Pawn|Input|AddControllerPitchInput Pitch))

(fn Moverse
  (params (Izquierda/Derecha :type Float%20%28double-precision%29) (Frente/Atras :type Float%20%28double-precision%29))
  (Pawn|Input|AddMovementInput (Transformation|GetActorRightVector) Izquierda/Derecha false)
  (Pawn|Input|AddMovementInput (Transformation|GetActorForwardVector) Frente/Atras false))

(fn Curar
  (params (Cantidad :type Float%20%28double-precision%29))
  (bind _output_get (Variables|Default|SetHP_Player (Math|Float|Clamp(Float) (+ (Variables|Default|GetHP_Player) Cantidad) 0.0 (Variables|Default|GetHP_Max_Player))))
  (Development|PrintString (Utilities|String|ToString(Float) _output_get)))