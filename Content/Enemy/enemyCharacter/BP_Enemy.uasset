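; BP_Enemy is an enemy character that chases the BP_Player actor, re-issuing AIMoveTo every tick.
; Overlapping its sphere launches the player character and applies damage.
; Incoming damage spawns a hit Niagara effect and removes at most one HP, gated by a DoOnce that resets after a short delay.
; The enemy destroys itself when HP reaches exactly zero.
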(event OnComponentBeginOverlap(Sphere)
  (params (OverlappedComponent :type Primitive%20Component%20Object%20Reference) (OtherActor :type Actor%20Object%20Reference) (OtherComp :type Primitive%20Component%20Object%20Reference) (OtherBodyIndex :type Integer) (bFromSweep :type Boolean) (SweepResult :type Hit%20Result%20Structure%20%28by%20ref%29))
  (bind _returnvalue (Game|GetPlayerCharacter 0))
  (if (== OtherActor _returnvalue)
    (Character|LaunchCharacter _returnvalue "10.000000,10.000000,50.000000" false false)
    (Game|Damage|ApplyDamage _returnvalue 1e+01 0 0)))

(event Custom|SpawnHit
  (Niagara|SpawnSystematLocation "/Game/SlashTrail_SoftTofu/Niagara/Dark/NS_Hit_Dark_OnceCopy.NS_Hit_Dark_OnceCopy" (Transformation|GetWorldLocation (Variables|Default|GetIdle))))

(event EventBeginPlay
  (bind _returnvalue (Actor|GetActorOfClass "/Game/Character/BP_Player.BP_Player_C"))
  (Variables|Default|SetPlayer _returnvalue))

(event Game|Damage|EventAnyDamage
  (params (Damage :type Float%20%28single-precision%29) (DamageType :type Damage%20Type%20Object%20Reference) (InstigatedBy :type Controller%20Object%20Reference) (DamageCauser :type Actor%20Object%20Reference))
  (Utilities|FlowControl|DoOnce false :!label _label
    (:Completed
      (CallFunction|SpawnHit)
      (bind _output_get (Variables|Default|SetHP (- (Variables|Default|GetHP) (Math|Float|Clamp(Float) Damage))))
      (Development|PrintString (Utilities|String|ToString(Float) _output_get))
      (if (== _output_get 0.0)
        (Actor|DestroyActor)
        (else
          (Utilities|FlowControl|Delay 0.2)
          (goto _label Reset))))))

(event EventTick
  (params (DeltaSeconds :type Float%20%28single-precision%29))
  (AI|AIMoveTo self "0, 0, 0" (Variables|Default|GetPlayer) 1e+02 false))

(fn ConstructionScript)