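; BP_EnemyRange is a ranged enemy that counts as a level objective through BPI_LevelManager.
; Tick faces the player, starts chasing within detection range, approaches at mid distance and retreats along a randomized direction when close.
; A looping timer, randomized per instance, fires BP_Proyectil at players in range.
; Hits play effects and remove at most one HP, with a DoOnce cooldown; zero HP completes the objective and destroys the actor.
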(event Custom|Disparar
  (bind _returnvalue (Transformation|GetActorLocation))
  (if (< (Transformation|GetDistanceTo (Variables|Default|GetPlayer)) 3e+03)
    (Game|SpawnActorfromClass "/Game/Enemy/enemyCharacter/BP_Proyectil.BP_Proyectil_C" (Math|Transform|MakeTransform _returnvalue (Math|Rotator|FindLookatRotation _returnvalue (Transformation|GetActorLocation (Game|GetPlayerCharacter 0))) "1.000000,1.000000,1.000000") "Undefined" "MultiplyWithRoot" 0 0)))

(event Custom|SpawnHit
  (Niagara|SpawnSystematLocation "/Game/SlashTrail_SoftTofu/Niagara/Dark/NS_Hit_Dark_Once.NS_Hit_Dark_Once" (Transformation|GetWorldLocation (Variables|Default|GetIdle)))
  (Audio|PlaySound2D "/Game/Character/art/_impacto._impacto" 1.0 1.0 0.0 0 0))

(event EventBeginPlay
  (bind _outactors (Actor|GetAllActorswithInterface "/Game/Features/LevelManager/BPI_LevelManager.BPI_LevelManager_C"))
  (Class|BPILevelManager|ObjectiveRegistered(Message) (Utilities|Array|Get(acopy) _outactors))
  (bind _returnvalue (Actor|GetActorOfClass "/Game/Character/BP_Player.BP_Player_C"))
  (Variables|Default|SetPlayer _returnvalue)
  (Utilities|Time|SetTimerbyEvent (delegate Custom|Disparar) (Math|Random|RandomFloatinRange 1.4 3.0) true))

(event Game|Damage|EventAnyDamage
  (params (Damage :type Float%20%28single-precision%29) (DamageType :type Damage%20Type%20Object%20Reference) (InstigatedBy :type Controller%20Object%20Reference) (DamageCauser :type Actor%20Object%20Reference))
  (Utilities|FlowControl|DoOnce false :!label _label
    (:Completed
      (CallFunction|SpawnHit)
      (bind _output_get (Variables|Default|SetHP (- (Variables|Default|GetHP) (Math|Float|Clamp(Float) Damage))))
      (Development|PrintString (Utilities|String|ToString(Float) _output_get))
      (if (== _output_get 0.0)
        (bind _outactors (Actor|GetAllActorswithInterface "/Game/Features/LevelManager/BPI_LevelManager.BPI_LevelManager_C"))
        (Class|BPILevelManager|ObjectiveCompleted(Message) (Utilities|Array|Get(acopy) _outactors))
        (Actor|DestroyActor)
        (else
          (Utilities|FlowControl|Delay 0.2)
          (goto _label Reset))))))

(event EventTick
  (params (DeltaSeconds :type Float%20%28single-precision%29))
  ;[0.15 0.15 0.15 0.5] Comment
  (Transformation|SetActorRotation (Math|Rotator|FindLookatRotation (Transformation|GetActorLocation) (Transformation|GetActorLocation (Variables|Default|GetPlayer))))
  (if (Variables|Default|GetIsChasing)
    (if (> (Transformation|GetDistanceTo (Variables|Default|GetPlayer)) 5e+02)
      (if (< (Transformation|GetDistanceTo (Variables|Default|GetPlayer)) 1.5e+03)
        (AI|AIMoveTo self "0, 0, 0" (Variables|Default|GetPlayer) 1e+02 false))
      (else
        (AI|AIMoveTo self (+ (* (Math|Vector|RotateVector (Math|Vector|Normalize (- (Transformation|GetActorLocation) (Transformation|GetActorLocation (Variables|Default|GetPlayer)))) (Math|Rotator|MakeRotator 0.0 (Math|Random|RandomFloatinRange -3e+01 3e+01) 0.0)) 3e+02) (Transformation|GetActorLocation)) 0 1e+02 false)))
    (elif (<= (Transformation|GetDistanceTo (Variables|Default|GetPlayer)) 3e+04)
      (Variables|Default|SetIsChasing true))))

(fn ConstructionScript)