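; Player controller that manages the main menu, pause menu and options widgets.
; IA_Pausar calls TogglePausar, which closes options if open, otherwise toggles game pause, pause widget visibility, input mode and cursor.
; Pause and options widgets are created on first use, cached, then shown or collapsed.
; OpenMainMenu only adds a new menu widget to the viewport; its UI-only input and cursor setup is disconnected.
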(event Custom|TogglePausar
  ;[0.15 0.15 0.15 0.5] Toggle Pausar
  (if (Variables|Default|GetbIsOptionsOpen)
    (CallFunction|CloseOptions)
    (elif (Game|IsGamePaused)
      (Widget|SetVisibility (Variables|Default|GetWBP_Pause_Ref) "Collapsed")
      (Game|SetGamePaused false)
      (Input|SetInputModeGameOnly self false)
      (Variables|Default|SetbShowMouseCursor false)
      (else
        (Utilities|IsValid (Variables|Default|GetWBP_Pause_Ref)
          (:Is%20Valid
            _)
          (:Is%20Not%20Valid
            (bind _returnvalue (UserInterface|CreateWidget "/Game/Shared/UI/PauseMenu/WBP_Pause.WBP_Pause_C" self))
            (bind _output_get (Variables|Default|SetWBP_Pause_Ref _returnvalue))
            (UserInterface|Viewport|AddtoViewport _output_get 0)))
        (Widget|SetVisibility (Variables|Default|GetWBP_Pause_Ref) "Visible")
        (Game|SetGamePaused true)
        (Input|SetInputModeGameandUI self (Variables|Default|GetWBP_Pause_Ref) "DoNotLock" true false)
        (Variables|Default|SetbShowMouseCursor true)))))

(event Custom|OpenOptions
  (Utilities|IsValid (Variables|Default|GetWBP_Options_Ref)
    (:Is%20Valid
      (Widget|SetVisibility (Variables|Default|GetWBP_Options_Ref) "Visible")
      (Variables|Default|SetbIsOptionsOpen true))
    (:Is%20Not%20Valid
      (bind _returnvalue (UserInterface|CreateWidget "/Game/Shared/UI/OptionsMenu/WBP_Options.WBP_Options_C" self))
      (bind _output_get (Variables|Default|SetWBP_Options_Ref _returnvalue))
      (UserInterface|Viewport|AddtoViewport _output_get 0)
      (Variables|Default|SetbIsOptionsOpen true))))

(event Custom|CloseOptions
  (Variables|/Script/UMG.Widget|SetVisibility (Variables|Default|GetWBP_Options_Ref) "Collapsed")
  (Variables|Default|SetbIsOptionsOpen false))

(event Custom|OpenMainMenu
  (bind _returnvalue (UserInterface|CreateWidget "/Game/Levels/MainMenu/UI/WBP_MainMenu.WBP_MainMenu_C"))
  (UserInterface|Viewport|AddtoViewport _returnvalue 0))

(event Input|EnhancedActionEvents|EnhancedInputActionIA_Pausar
  (params (ActionValue :type Boolean) (ElapsedSeconds :type Float%20%28double-precision%29) (TriggeredSeconds :type Float%20%28double-precision%29) (InputAction :type Input%20Action%20Object%20Reference :default "/Game/Character/Input/Actions/IA_Pausar.IA_Pausar"))
  ;[0.15 0.15 0.15 0.5] Toggle Pausar
  (CallFunction|TogglePausar))

(fn ConstructionScript)