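; BP_TriggerButton is a one-shot button actor that explodes when it is hit or takes any damage.
; Hit and AnyDamage both feed the Explode event, where a Triggered flag lets the effect run only once.
; Explode spawns a particle effect and plays a sound at the actor's location, then hides the static mesh and disables its collision without destroying the actor.
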(event Custom|Explode
  (bind _returnvalue (Transformation|GetActorLocation))
  (if (not (Variables|Default|GetbTriggered))
    (Variables|Default|SetbTriggered true)
    (Effects|SpawnEmitteratLocation "/Engine/Tutorial/SubEditors/TutorialAssets/TutorialParticleSystem.TutorialParticleSystem" _returnvalue)
    (Audio|PlaySoundatLocation "/Engine/EditorSounds/GamePreview/PossessPlayer_Cue.PossessPlayer_Cue" _returnvalue "0, 0, 0" 1.0 1.0 0.0 0 0 0 0)
    (Rendering|SetVisibility (Variables|Default|GetStaticMesh) false false)
    (Collision|SetCollisionEnabled (Variables|Default|GetStaticMesh) "NoCollision")))

(event EventBeginPlay)

(event Collision|EventActorBeginOverlap
  (params (OtherActor :type Actor%20Object%20Reference)))

(event EventTick
  (params (DeltaSeconds :type Float%20%28single-precision%29)))

(event Collision|EventHit
  (params (MyComp :type Primitive%20Component%20Object%20Reference) (Other :type Actor%20Object%20Reference) (OtherComp :type Primitive%20Component%20Object%20Reference) (bSelfMoved :type Boolean) (HitLocation :type Vector :default "0, 0, 0") (HitNormal :type Vector :default "0, 0, 0") (NormalImpulse :type Vector :default "0, 0, 0") (Hit :type Hit%20Result%20Structure%20%28by%20ref%29))
  (CallFunction|Explode))

(event Game|Damage|EventAnyDamage
  (params (Damage :type Float%20%28single-precision%29) (DamageType :type Damage%20Type%20Object%20Reference) (InstigatedBy :type Controller%20Object%20Reference) (DamageCauser :type Actor%20Object%20Reference))
  (CallFunction|Explode))

(fn ConstructionScript)