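; An actor Blueprint for a membrane that bursts once, either when its linked trigger button fires or when Tocar is called.
; On BeginPlay it binds Explode to the button's triggered event.
; Explode is guarded by a Triggered flag, then spawns a particle effect and a sound at its location, hides the mesh and destroys the actor.
; A node that disables mesh collision is left unconnected.
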(event Custom|Explode
  (bind _returnvalue (Transformation|GetActorLocation))
  (if (not (Variables|Default|GetbTriggered))
    (Variables|Default|SetbTriggered true)
    (Effects|SpawnEmitteratLocation "/Engine/Tutorial/SubEditors/TutorialAssets/TutorialParticleSystem.TutorialParticleSystem" _returnvalue)
    (Audio|PlaySoundatLocation "/Engine/EditorSounds/GamePreview/PossessPlayer_Cue.PossessPlayer_Cue" _returnvalue "0, 0, 0" 1.0 1.0 0.0 0 0 0 0)
    (Rendering|SetVisibility (Variables|Default|GetStaticMesh) false true)
    (Actor|DestroyActor)))

(event EventBeginPlay
  (EventDispatchers|BindEventtoOnButtonTriggered (Variables|Default|GetTriggerButtonRef) (delegate Custom|Explode)))

(event EventTocar
  (CallFunction|Explode))

(fn ConstructionScript)