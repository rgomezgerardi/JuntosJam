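; BP_ZonaCuracion is a healing zone with a limited health pool that plays a sound and spawns a Niagara effect on spawn.
; A BP_Player entering OrbeSphere starts a looping 0.1-second timer, and leaving stops healing.
; Each active tick drains the pool by a per-second rate, passes the remaining pool value to the player's Curar, and destroys the zone when empty.
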(event OnComponentBeginOverlap(OrbeSphere)
  (params (OverlappedComponent :type Primitive%20Component%20Object%20Reference) (OtherActor :type Actor%20Object%20Reference) (OtherComp :type Primitive%20Component%20Object%20Reference) (OtherBodyIndex :type Integer) (bFromSweep :type Boolean) (SweepResult :type Hit%20Result%20Structure%20%28by%20ref%29))
  (bind _asbp_player (Utilities|Casting|CastToBP_Player OtherActor))
  (CallFunction|EmpezarCurar _asbp_player)
  (Audio|PlaySound2D "/Game/Character/art/_burbuja-inmunidad._burbuja-inmunidad" 1.0 1.0 0.0 0 0))

(event OnComponentEndOverlap(OrbeSphere)
  (params (OverlappedComponent :type Primitive%20Component%20Object%20Reference) (OtherActor :type Actor%20Object%20Reference) (OtherComp :type Primitive%20Component%20Object%20Reference) (OtherBodyIndex :type Integer))
  (Utilities|Casting|CastToBP_Player OtherActor)
  (CallFunction|DetenerCurar))

(event Custom|EmpezarCurar
  (params (Jugador :type BP%20Player%20Object%20Reference))
  (if (> (Variables|Default|GetVidaRestante) 0.0)
    (Variables|Default|SetJugadorActual Jugador)
    (Variables|Default|SetbActivo true)
    (Utilities|Time|SetTimerbyEvent (delegate Custom|TickCurar) 0.1 true)
    (Variables|Default|SetTimerHandle_Curar "")))

(event Custom|TickCurar
  (if (and (Variables|Default|GetbActivo) (> (Variables|Default|GetVidaRestante) 0.0))
    (Utilities|FlowControl|Sequence
      (:then_0
        (bind _output_get (Variables|Default|SetVidaRestante (- (Variables|Default|GetVidaRestante) (Math|Float|Min(Float) (* (Variables|Default|GetVidaPorSegundo) 0.1) (Variables|Default|GetVidaRestante)))))
        (Default|Curar (Variables|Default|GetJugadorActual) _output_get)
        (if (<= (Variables|Default|GetVidaRestante) 0.0)
          (CallFunction|DetenerCurar)
          (Actor|DestroyActor)))
      (:then_1
        (Utilities|FlowControl|DoOnce false)))))

(event Custom|DetenerCurar
  (Utilities|Time|ClearandInvalidateTimerbyHandle (Variables|Default|GetTimerHandle_Curar))
  (Variables|Default|SetbActivo false))

(event EventBeginPlay
  (Variables|Default|SetVidaRestante (Variables|Default|GetVidaTotal))
  (Audio|PlaySound2D "/Game/Character/art/_impacto-brbuja._impacto-brbuja" 1.0 1.0 0.0 0 0)
  (Niagara|SpawnSystematLocation "/Game/SlashTrail_SoftTofu/Niagara/Dark/NS_SlashTrail_Dark_Loop.NS_SlashTrail_Dark_Loop" (Transformation|GetWorldLocation (Variables|Default|GetDefaultSceneRoot))))

(fn ConstructionScript)