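; BP_Cupula is a dome actor that breaks once enough trigger buttons have fired, activating a Boss's movement.
; On BeginPlay it stores the number of referenced buttons and binds each one's triggered event to Explode.
; Each Explode call, also reachable through Tocar, increments a counter.
; At the total it enables the Boss's move flag, then plays a one-time particle and sound, hides its sphere and destroys itself.
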(event Custom|Explode
  (bind _returnvalue (Transformation|GetActorLocation))
  (Math|Integer|IncrementInt (Variables|Default|GetExplodesCount)
    (:%20%20
      (if (>= (Variables|Default|GetExplodesCount) (Variables|Default|GetTriggerButtonRefTotal))
        (Variables|/Game/Enemy/Boss/BP_Boss.BP_Boss_C|SetActivateMove (Variables|Default|GetBoss) true)
        (if (not (Variables|Default|GetbTriggered))
          (Variables|Default|SetbTriggered true)
          (Effects|SpawnEmitteratLocation "/Engine/Tutorial/SubEditors/TutorialAssets/TutorialParticleSystem.TutorialParticleSystem" _returnvalue)
          (Audio|PlaySoundatLocation "/Engine/EditorSounds/GamePreview/PossessPlayer_Cue.PossessPlayer_Cue" _returnvalue "0, 0, 0" 1.0 1.0 0.0 0 0 0 0)
          (Rendering|SetVisibility (Variables|Default|GetSphere) false true)
          (Actor|DestroyActor))))))

(event EventBeginPlay
  (Variables|Default|SetTriggerButtonRefTotal (Utilities|Array|Length (Variables|Default|GetTriggerButtonRef)))
  (EventDispatchers|BindEventtoOnButtonTriggered (Variables|Default|GetTriggerButtonRef) (delegate Custom|Explode)))

(event EventTocar
  (CallFunction|Explode))

(fn ConstructionScript)