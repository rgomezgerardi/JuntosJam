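; BP_DialogueManager is an actor that starts dialogue and shows it on screen in a WBP_DialogueBox widget.
; StartDialogue takes a row name and sets an active flag to reject overlapping requests; nothing in this Blueprint clears that flag.
; PlayDialogue creates and stores the widget, adds it to the viewport, then fills in speaker and content from the matching DTDialogue data table row.
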(event EventBeginPlay)

(event Collision|EventActorBeginOverlap
  (params (OtherActor :type Actor%20Object%20Reference)))

(event EventTick
  (params (DeltaSeconds :type Float%20%28single-precision%29)))

(event EventStartDialogue
  (params (RowName :type Name :default "None"))
  (if (Variables|Default|GetIsDialogueActive)
    (Development|PrintString "There is already an active dialogue.")
    (else
      (Variables|Default|SetIsDialogueActive true)
      (CallFunction|PlayDialogue RowName))))

(fn ConstructionScript)

(fn PlayDialogue
  (params (RowName :type Name))
  (bind _returnvalue (UserInterface|CreateWidget "/Game/Features/DialogueSystem/WBP_DialogueBox.WBP_DialogueBox_C"))
  (bind _output_get (Variables|Default|SetActiveWidget _returnvalue))
  (UserInterface|Viewport|AddtoViewport _output_get 0)
  (bind _returnvalue_2 (Utilities|GetDataTableRow (Variables|Default|GetDT_Dialogue) RowName)
    (:then
      (Default|UpdateText (Variables|Default|GetActiveWidget) (.Speaker (Utilities|Struct|BreakS_DialogueData _returnvalue_2)) (.Content (Utilities|Struct|BreakS_DialogueData _returnvalue_2))))))