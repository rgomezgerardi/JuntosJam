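; BP_LevelManager runs level flow: objective progress, checkpoint respawns and the scripted opening scene.
; Objective register/complete events update counters and send the completion ratio to the KidStatus widget, created on BeginPlay, via BPI_KidStatus.
; On death, it resets player HP and moves the player to the last saved checkpoint location.
; TriggerScene chains dialogue lines with camera blends to a level camera and back, disabling player input throughout.
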(event Custom|TriggerScene
  (params (NewParam :type Name))
  (switch name NewParam
    (:1
      (Input|DisableInput (Game|Player|GetPlayerPawn 0) (Game|GetPlayerController 0))
      (Utilities|PlaySyncDialogue (Variables|Default|GetDialogueManager) "1" false 0.0
        (:Completed
          (Utilities|FlowControl|Delay 0.2)
          (Utilities|PlaySyncDialogue (Variables|Default|GetDialogueManager) "2" false 0.0
            (:Completed
              (Utilities|FlowControl|Delay 0.2)
              (Game|Player|SetViewTargetwithBlend (Game|GetPlayerController 0) (Utilities|Array|Get(acopy) (Variables|Default|GetLevelCameras)) 1.0 "VTBlend_Linear" 0.0 false)
              (Utilities|FlowControl|Delay 0.2)
              (Utilities|PlaySyncDialogue (Variables|Default|GetDialogueManager) "3" false 0.0
                (:Completed
                  (Utilities|FlowControl|Delay 0.2)
                  (Utilities|PlaySyncDialogue (Variables|Default|GetDialogueManager) "4" false 0.0
                    (:Completed
                      (Utilities|FlowControl|Delay 0.2)
                      (bind _returnvalue (Actor|GetActorOfClass "/Game/Character/BP_Player.BP_Player_C"))
                      (Game|Player|SetViewTargetwithBlend (Game|GetPlayerController 0) _returnvalue 0.5 "VTBlend_Linear" 0.0 false)
                      (Utilities|FlowControl|Delay 0.2)
                      (Utilities|PlaySyncDialogue (Variables|Default|GetDialogueManager) "5" false 0.0
                        (:Completed
                          (Input|EnableInput (Game|Player|GetPlayerPawn 0) (Game|GetPlayerController 0)))))))))))))))

(event EventBeginPlay
  ;[0.15 0.15 0.15 0.5] Inicialización
  (bind _returnvalue (Actor|GetActorOfClass "/Game/Character/BP_Player.BP_Player_C"))
  (Variables|Default|SetPlayer _returnvalue)
  (bind _returnvalue_2 (UserInterface|CreateWidget "/Game/Features/HUD/KidStatus/WBP_KidStatus.WBP_KidStatus_C"))
  (bind _output_get (Variables|Default|SetKidStatus _returnvalue_2))
  (UserInterface|Viewport|AddtoViewport _output_get 0)
  (CallFunction|TriggerScene "1"))

(event EventUpdatePlayerLocation
  (params (Location :type Vector :default "0, 0, 0"))
  (Variables|Default|SetLastCheckpointLocation Location))

(event EventObjectiveCompleted
  ;[0.15 0.15 0.15 0.5] Al destruir a un objetivo, calcular progreso (objetivos completados / objetivos totales) y enviar al WBP_KidStatus
  (bind _result (Math|Float|IncrementFloat (Variables|Default|GetCompletedObjectives))
    (:%20%20
      (Development|PrintString (Utilities|String|Append (Utilities|String|Append (Utilities|String|ToString(Float) _result) " / ") (Utilities|String|ToString(Float) (Variables|Default|GetObjectives))) true true "(R=0.157417,G=1.000000,B=0.000000,A=1.000000)" 1e+01)
      (bind _foundwidgets (Class|WidgetBlueprintLibrary|GetAllWidgetswithInterface "/Game/Features/HUD/KidStatus/BPI_KidStatus.BPI_KidStatus_C" false))
      (Class|BPIKidStatus|SetProgress(Message) (Utilities|Array|Get(acopy) _foundwidgets) (/ (Variables|Default|GetCompletedObjectives) (Variables|Default|GetObjectives))))))

(event EventObjectiveRegistered
  (Math|Float|IncrementFloat (Variables|Default|GetObjectives)
    (:%20%20
      (bind _foundwidgets (Class|WidgetBlueprintLibrary|GetAllWidgetswithInterface "/Game/Features/HUD/KidStatus/BPI_KidStatus.BPI_KidStatus_C" false))
      (Class|BPIKidStatus|SetProgress(Message) (Utilities|Array|Get(acopy) _foundwidgets) (/ (Variables|Default|GetCompletedObjectives) (Variables|Default|GetObjectives))))))

(event EventPlayerIsDead
  ;[0.15 0.15 0.15 0.5] Respawn con Checkpoint
  (Variables|/Game/Character/BP_Player.BP_Player_C|SetHP_Player (Variables|Default|GetPlayer) 1e+01)
  (Transformation|SetActorLocation (Variables|Default|GetPlayer) (Variables|Default|GetLastCheckpointLocation) false false))

(fn ConstructionScript)